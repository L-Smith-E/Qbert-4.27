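; BallSpawns is an enemy spawner Blueprint that adds either a green or red variant as a child actor at construction time.
; The Construction Script calls SetSpawns, an empty stub here, then randomly runs GreenSpawn or RedSpawn.
; Both place a Child Actor Component at a SpawnPoints transform, but their reversed random range (last index to zero) resolves to the last point.
; The event graph is unused.
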(event EventBeginPlay)

(event Collision|EventActorBeginOverlap
  (params (OtherActor :type Actor%20Object%20Reference)))

(event EventTick
  (params (DeltaSeconds :type Float%20%28single-precision%29)))

(fn ConstructionScript
  (CallFunction|SetSpawns)
  (switch int (Math|Random|RandomIntegerinRange 0 1)
    (:0
      (CallFunction|GreenSpawn))
    (:1
      (CallFunction|RedSpawn))))

(fn SetSpawns)

(fn GreenSpawn
  (bind _spawnpoints (Variables|Default|GetSpawnPoints))
  (AddComponent|AddChildActorComponent false (Utilities|Array|Get(acopy) _spawnpoints (Math|Random|RandomIntegerinRange (Utilities|Array|LastIndex _spawnpoints) 0))))

(fn RedSpawn
  (bind _spawnpoints (Variables|Default|GetSpawnPoints))
  (AddComponent|AddChildActorComponent false (Utilities|Array|Get(acopy) _spawnpoints (Math|Random|RandomIntegerinRange (Utilities|Array|LastIndex _spawnpoints) 0))))