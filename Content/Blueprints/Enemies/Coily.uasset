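; Coily is a Q*bert enemy that chases the player in diagonal hops and costs lives on overlap.
; Tick compares Y and Z against Qbert, cycling a delayed MultiGate that, after an initial down-right hop, teleports the mesh by fixed offsets.
; The game mode's green-ball flag delays movement five seconds.
; Overlapping Offlevel destroys Coily and all red and green balls, then awards points through the game mode.
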(event OnComponentBeginOverlap(Damage)
  (params (OverlappedComponent :type Primitive%20Component%20Object%20Reference) (OtherActor :type Actor%20Object%20Reference) (OtherComp :type Primitive%20Component%20Object%20Reference) (OtherBodyIndex :type Integer) (bFromSweep :type Boolean) (SweepResult :type Hit%20Result%20Structure%20%28by%20ref%29))
  ;[1 1 1] Damage Qbert
  (bind _asqbert (Utilities|Casting|CastToQbert OtherActor))
  (Default|LivesSystem _asqbert (Variables|Default|Get-Life)))

(event OnComponentBeginOverlap(deathCap)
  (params (OverlappedComponent :type Primitive%20Component%20Object%20Reference) (OtherActor :type Actor%20Object%20Reference) (OtherComp :type Primitive%20Component%20Object%20Reference) (OtherBodyIndex :type Integer) (bFromSweep :type Boolean) (SweepResult :type Hit%20Result%20Structure%20%28by%20ref%29))
  ;[1 1 1] Coily Death State
  (Utilities|Casting|CastToOfflevel OtherActor)
  (Actor|DestroyActor)
  (bind _asred_ball (Utilities|Casting|CastToRedBallClass "/Game/Blueprints/Enemies/RedBall.RedBall_C"))
  (bind _outactors (Actor|GetAllActorsOfClass _asred_ball))
  (Actor|DestroyActor _outactors)
  (bind _asgreen_ball (Utilities|Casting|CastToGreenBallClass "/Game/Blueprints/Enemies/GreenBall.GreenBall_C"))
  (bind _outactors_2 (Actor|GetAllActorsOfClass _asgreen_ball))
  (Actor|DestroyActor _outactors_2)
  (bind _asqbert_gm_bp (Utilities|Casting|CastToQbertGM_BP (Game|GetGameMode)))
  (Default|AddPoints _asqbert_gm_bp (Variables|Default|GetCoilyPts))
  (Development|PrintString "CoilyPts:500" true true "(R=0.262841,G=1.000000,B=0.418989,A=1.000000)"))

(event Custom|Movement
  (params (Movement :type Transform))
  (bind _staticmesh (Variables|Default|GetStaticMesh))
  ;[1 1 1] Movement
  (Transformation|SetWorldTransform _staticmesh (Math|Transform|MakeTransform (+ (.location (Transformation|GetWorldTransform _staticmesh)) (.location Movement)) "1.000000,1.000000,1.000000" "1,1,1") false true))

(event EventBeginPlay)

(event Collision|EventActorBeginOverlap
  (params (OtherActor :type Actor%20Object%20Reference)))

(event EventTick
  (params (DeltaSeconds :type Float%20%28single-precision%29))
  ;[1 1 1] Movement AI
  (bind _asqbert (Utilities|Casting|CastToQbert (Game|Player|GetPlayerPawn 0)))
  (bind _ascoily (Utilities|Casting|CastToCoily self))
  (Variables|Default|SetLeft (< (.y (Transformation|GetWorldLocation (Variables|/Game/Blueprints/Qbert/Qbert.Qbert_C|GetStaticMesh _asqbert))) (.y (Transformation|GetWorldLocation (Variables|Coily_C|GetStaticMesh _ascoily)))))
  (Variables|Default|SetRight (> (.y (Transformation|GetWorldLocation (Variables|/Game/Blueprints/Qbert/Qbert.Qbert_C|GetStaticMesh _asqbert))) (.y (Transformation|GetWorldLocation (Variables|Coily_C|GetStaticMesh _ascoily)))))
  (Variables|Default|SetUp (> (.z (Transformation|GetWorldLocation (Variables|/Game/Blueprints/Qbert/Qbert.Qbert_C|GetStaticMesh _asqbert))) (.z (Transformation|GetWorldLocation (Variables|Coily_C|GetStaticMesh _ascoily)))))
  (Variables|Default|SetDown (< (.z (Transformation|GetWorldLocation (Variables|/Game/Blueprints/Qbert/Qbert.Qbert_C|GetStaticMesh _asqbert))) (.z (Transformation|GetWorldLocation (Variables|Coily_C|GetStaticMesh _ascoily)))))
  ;;[1 1 1] If Green ball is hit delay movement
  (bind _asqbert_gm_bp (Utilities|Casting|CastToQbertGM_BP (Game|GetGameMode)))
  (if (Variables|/Game/Blueprints/QbertGM_BP.QbertGM_BP_C|GetGreenB _asqbert_gm_bp)
    (Utilities|FlowControl|Delay 5.0)
    (Utilities|FlowControl|MultiGate false true 0 :!label _label
      (:Out%200
        (Utilities|FlowControl|Delay 3.0)
        (Utilities|FlowControl|DoN 1
          (:Exit
            (Variables|Default|SetCoils true)
            ;[1 1 1] down right
            (CallFunction|Movement (Math|Transform|MakeTransform "-71.000000,71.000000,-100.000000" "1.000000,1.000000,1.000000" "1,1,1") :!label _label_2))))
      (:Out%201
        (Utilities|FlowControl|Delay 0.05)
        (if (Variables|Default|GetCoils)
          (if (and (Variables|Default|GetRight) (Variables|Default|GetDown))
            (Utilities|FlowControl|Delay (Variables|Default|GetTick))
            (goto _label_2))))
      (:Out%202
        (Utilities|FlowControl|Delay 0.05)
        (if (Variables|Default|GetCoils)
          ;[1 1 1] Down-Left Movement
          (if (and (Variables|Default|GetLeft) (Variables|Default|GetDown))
            (Utilities|FlowControl|Delay (Variables|Default|GetTick))
            (CallFunction|Movement (Math|Transform|MakeTransform "-71.000000,-71.000000,-100.000000" "1.000000,1.000000,1.000000" "1,1,1")))))
      (:Out%203
        (Utilities|FlowControl|Delay 0.05)
        (if (Variables|Default|GetCoils)
          ;[1 1 1] Up-Left Movement
          (if (and (Variables|Default|GetLeft) (Variables|Default|GetUp))
            (Utilities|FlowControl|Delay (Variables|Default|GetTick))
            (CallFunction|Movement (Math|Transform|MakeTransform "71.000000,-71.000000,100.000000" "1.000000,1.000000,1.000000" "1,1,1")))))
      (:Out%204
        (Utilities|FlowControl|Delay 0.05)
        (if (Variables|Default|GetCoils)
          ;[1 1 1] Up-Right Movement
          (if (and (Variables|Default|GetRight) (Variables|Default|GetUp))
            (Utilities|FlowControl|Delay (Variables|Default|GetTick))
            (CallFunction|Movement (Math|Transform|MakeTransform "71.000000,71.000000,100.000000" "1.000000,1.000000,1.000000" "1,1,1"))))))
    (elif true
      (goto _label))))

(fn ConstructionScript)