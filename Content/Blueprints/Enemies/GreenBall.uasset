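; Green ball pickup for a Q*bert-style game that hops down the level and rewards Qbert on contact.
; A Delay on Tick paces fixed teleport steps of the Sphere, always down-right; the other three directions are unconnected.
; Qbert overlapping Sphere1 destroys the ball, adds points and sets the GreenB flag in QbertGM_BP.
; The KillActor component destroys it upon overlapping an Offlevel actor.
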(event OnComponentBeginOverlap(Sphere1)
  (params (OverlappedComponent :type Primitive%20Component%20Object%20Reference) (OtherActor :type Actor%20Object%20Reference) (OtherComp :type Primitive%20Component%20Object%20Reference) (OtherBodyIndex :type Integer) (bFromSweep :type Boolean) (SweepResult :type Hit%20Result%20Structure%20%28by%20ref%29))
  ;[1 1 1] Add Points
  (Utilities|Casting|CastToQbert OtherActor)
  (Actor|DestroyActor)
  (bind _asqbert_gm_bp (Utilities|Casting|CastToQbertGM_BP (Game|GetGameMode)))
  (Default|AddPoints _asqbert_gm_bp (Variables|Default|Get100+))
  (Variables|/Game/Blueprints/QbertGM_BP.QbertGM_BP_C|SetGreenB _asqbert_gm_bp true))

(event OnComponentBeginOverlap(KillActor)
  (params (OverlappedComponent :type Primitive%20Component%20Object%20Reference) (OtherActor :type Actor%20Object%20Reference) (OtherComp :type Primitive%20Component%20Object%20Reference) (OtherBodyIndex :type Integer) (bFromSweep :type Boolean) (SweepResult :type Hit%20Result%20Structure%20%28by%20ref%29))
  ;[1 1 1] OffLevel
  (Utilities|Casting|CastToOfflevel OtherActor)
  (Actor|DestroyActor))

(event EventBeginPlay)

(event Collision|EventActorBeginOverlap
  (params (OtherActor :type Actor%20Object%20Reference)))

(event EventTick
  (params (DeltaSeconds :type Float%20%28single-precision%29))
  (bind _sphere (Variables|Default|GetSphere))
  (Utilities|FlowControl|Delay 2.55)
  ;[1 1 1] Down-Right Movement
  (if true
    (Utilities|FlowControl|Delay (Variables|Default|GetTick))
    (Transformation|SetWorldTransform _sphere (Math|Transform|MakeTransform (+ (.location (Transformation|GetWorldTransform _sphere)) "-71.000000,71.000000,-100.000000") "1.000000,1.000000,1.000000" "0.750000,0.750000,0.750000") false true)))

(fn ConstructionScript)