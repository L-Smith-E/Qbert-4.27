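; Red ball enemy for a Q*bert-style game that hops down the level and costs Qbert a life on contact.
; Tick chains delays to teleport the Sphere by a fixed down-right step; the other three diagonal moves are present but disconnected.
; The Damage overlap calls Qbert's LivesSystem, and the KillActor overlap destroys the ball when it touches an Offlevel actor.
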(event OnComponentBeginOverlap(Damage)
  (params (OverlappedComponent :type Primitive%20Component%20Object%20Reference) (OtherActor :type Actor%20Object%20Reference) (OtherComp :type Primitive%20Component%20Object%20Reference) (OtherBodyIndex :type Integer) (bFromSweep :type Boolean) (SweepResult :type Hit%20Result%20Structure%20%28by%20ref%29))
  ;[1 1 1] Damage Qbert
  (bind _asqbert (Utilities|Casting|CastToQbert OtherActor))
  (Default|LivesSystem _asqbert (Variables|Default|Get-Life)))

(event OnComponentBeginOverlap(KillActor)
  (params (OverlappedComponent :type Primitive%20Component%20Object%20Reference) (OtherActor :type Actor%20Object%20Reference) (OtherComp :type Primitive%20Component%20Object%20Reference) (OtherBodyIndex :type Integer) (bFromSweep :type Boolean) (SweepResult :type Hit%20Result%20Structure%20%28by%20ref%29))
  (Utilities|Casting|CastToOfflevel OtherActor)
  (Actor|DestroyActor))

(event Custom|Movement
  (params (Movement :type Transform))
  (bind _sphere (Variables|Default|GetSphere))
  ;[1 1 1] Movement
  (Transformation|SetWorldTransform _sphere (Math|Transform|MakeTransform (+ (.location (Transformation|GetWorldTransform _sphere)) (.location Movement)) "1.000000,1.000000,1.000000" "0.750000,0.750000,0.750000") false true))

(event EventBeginPlay)

(event Collision|EventActorBeginOverlap
  (params (OtherActor :type Actor%20Object%20Reference)))

(event EventTick
  (params (DeltaSeconds :type Float%20%28single-precision%29))
  (Utilities|FlowControl|Delay 2.55)
  ;[1 1 1] down right
  (if true
    (Utilities|FlowControl|Delay (Variables|Default|GetTick))
    (CallFunction|Movement (Math|Transform|MakeTransform "-71.000000,71.000000,-100.000000" "1.000000,1.000000,1.000000" "1.000000,1.000000,1.000000"))))

(fn ConstructionScript)