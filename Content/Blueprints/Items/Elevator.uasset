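; Elevator actor for a Q*bert game that starts moving when Qbert overlaps its box.
; On overlap it sets Qbert's Child flag, teleports his mesh by a fixed offset, and sets the Elevators flag on QbertGM_BP.
; MoveElevator plays a timeline, rate-scaled by Duration, that moves the actor along the referenced track's spline from start to end.
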(event OnComponentBeginOverlap(Box)
  (params (OverlappedComponent :type Primitive%20Component%20Object%20Reference) (OtherActor :type Actor%20Object%20Reference) (OtherComp :type Primitive%20Component%20Object%20Reference) (OtherBodyIndex :type Integer) (bFromSweep :type Boolean) (SweepResult :type Hit%20Result%20Structure%20%28by%20ref%29))
  ;[1 1 1] Move Qbert on Elevator Overlap
  (bind _asqbert (Utilities|Casting|CastToQbert OtherActor))
  (Variables|/Game/Blueprints/Qbert/Qbert.Qbert_C|SetChild _asqbert true)
  (CallFunction|MoveElevator)
  (Transformation|SetWorldTransform (Variables|/Game/Blueprints/Qbert/Qbert.Qbert_C|GetStaticMesh _asqbert) (Math|Transform|MakeTransform (+ (.location (Transformation|GetWorldTransform (Variables|/Game/Blueprints/Qbert/Qbert.Qbert_C|GetStaticMesh _asqbert))) "352.000000,-495.000000,500.000000") "0, 0, 0" "0.250000,0.250000,0.250000") false true)
  (Variables|/Game/Blueprints/Qbert/Qbert.Qbert_C|SetChild _asqbert true)
  (bind _asqbert_gm_bp (Utilities|Casting|CastToQbertGM_BP (Game|GetGameMode)))
  (Variables|/Game/Blueprints/QbertGM_BP.QbertGM_BP_C|SetElevators _asqbert_gm_bp true))

(event Custom|Move%20Elevator
  ;[1 1 1] Move Elevator
  (Components|Timeline|SetPlayRate (Variables|Default|GetMovement) (/ 1.0 (Variables|Default|GetDuration)))
  (bind _alpha (Timeline|Movement Play)
    (:Update
      (Variables|Default|SetAlpha _alpha)
      (Transformation|SetActorLocationAndRotation (Spline|GetLocationatDistanceAlongSpline (Variables|/Game/Blueprints/Items/ETrack.ETrack_C|GetESpline (Variables|Default|GetTrackRef)) (Math|Float|Lerp 0.0 (Spline|GetSplineLength (Variables|/Game/Blueprints/Items/ETrack.ETrack_C|GetESpline (Variables|Default|GetTrackRef))) (Variables|Default|GetAlpha)) "World") "0, 0, 0"))))

(event Collision|EventActorBeginOverlap
  (params (OtherActor :type Actor%20Object%20Reference)))

(event EventTick
  (params (DeltaSeconds :type Float%20%28single-precision%29)))

(fn ConstructionScript)