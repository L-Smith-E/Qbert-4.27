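; Q*bert-style platform tile that changes colour and awards score the first time the player lands on it.
; When Qbert overlaps the Plane while it shows the blue material, it swaps to the new material and adds points and a tally to QbertGM_BP.
; WinMatChange starts a looping timer that randomly cycles materials from MATArray, adds the win screen widget and shows the mouse cursor.
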(event OnComponentBeginOverlap(Plane)
  (params (OverlappedComponent :type Primitive%20Component%20Object%20Reference) (OtherActor :type Actor%20Object%20Reference) (OtherComp :type Primitive%20Component%20Object%20Reference) (OtherBodyIndex :type Integer) (bFromSweep :type Boolean) (SweepResult :type Hit%20Result%20Structure%20%28by%20ref%29))
  ;[1 1 1] Change Colour/Add Score/AddTally
  (Utilities|Casting|CastToQbert OtherActor)
  (if (== (Variables|Default|GetBlue%20MAT) (Rendering|Material|GetMaterial (Variables|Default|GetPlane) 0))
    (Rendering|Material|SetMaterial (Variables|Default|GetPlane) 0 (Variables|Default|GetPlane_New_Material))
    (bind _asqbert_gm_bp (Utilities|Casting|CastToQbertGM_BP (Game|GetGameMode)))
    (Default|AddPoints _asqbert_gm_bp (Variables|Default|GetTarget%20Score))
    (Default|AddTally _asqbert_gm_bp)))

(event Custom|WinMatChange
  (Utilities|Time|SetTimerbyFunctionName 0 "Change Colour" 0.5 true)
  (bind _returnvalue (UserInterface|CreateWidget "/Game/Blueprints/UI/WinScreen.WinScreen_C"))
  (UserInterface|Viewport|AddtoViewport _returnvalue 0)
  (Variables|/Script/Engine.PlayerController|SetbShowMouseCursor (Game|GetPlayerController 0) true))

(event EventBeginPlay)

(event Collision|EventActorBeginOverlap
  (params (OtherActor :type Actor%20Object%20Reference)))

(event EventTick
  (params (DeltaSeconds :type Float%20%28single-precision%29)))

(fn ConstructionScript)

(fn ChangeColour
  (bind _matarray (Variables|Default|GetMATArray))
  (Rendering|Material|SetMaterial (Variables|Default|GetPlane) 0 (Utilities|Array|Get(acopy) _matarray (Math|Random|RandomInteger (+ (Utilities|Array|LastIndex _matarray) 1)))))