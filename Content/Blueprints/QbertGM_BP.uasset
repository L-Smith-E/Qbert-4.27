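; QbertGM_BP is the Q*bert game manager Blueprint that tracks score and the platform win condition.
; AddPoints accumulates the score, while AddTally counts platforms until the target total is reached, both printing debug text.
; Reaching the target shows the WinScreen widget with the mouse cursor, pauses the game and awards a bonus if Elevators is false.
; A GameOver call and a Points reset are present but never run.
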(event Custom|AddPoints
  (params (Add%20Score :type Integer))
  ;[1 1 1] Scoring System
  (bind _output_get (Variables|Default|SetTargetScore (+ Add%20Score (Variables|Default|GetTargetScore))))
  (Development|PrintString (Utilities|String|Append "Current Points: " (Utilities|String|ToString(Integer) _output_get))))

(event Custom|Add%20Tally
  ;[1 1 1] Win Condition
  (bind _output_get (Variables|Default|SetTally (+ (Variables|Default|GetTally) (Variables|Default|Get1))))
  (Development|PrintString (Utilities|String|Append "Platform Tally: " (Utilities|String|ToString(Integer) _output_get)) true true "(R=1.000000,G=0.024480,B=0.000000,A=1.000000)")
  (if (== (Variables|Default|GetTally) (Variables|Default|GetTTally))
    (Development|PrintString "Win" true true "(R=1.000000,G=0.313331,B=0.000000,A=1.000000)")
    (CallFunction|GameWin)
    (Game|SetGamePaused true)
    (if (not (Variables|Default|GetElevators))
      (CallFunction|AddPoints 100))))

(event Custom|GameWin
  ;[1 1 1] Win Condition
  (bind _returnvalue (UserInterface|CreateWidget "/Game/Blueprints/UI/WinScreen.WinScreen_C"))
  (UserInterface|Viewport|AddtoViewport _returnvalue 0)
  (Variables|/Script/Engine.PlayerController|SetbShowMouseCursor (Game|GetPlayerController 0) true))

(event EventBeginPlay)

(event EventTick
  (params (DeltaSeconds :type Float%20%28single-precision%29)))

(fn ConstructionScript)